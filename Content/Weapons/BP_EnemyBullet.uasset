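; BP_EnemyBullet is an enemy projectile that damages the player on overlap.
; Tick moves it along its forward vector by Speed without sweeping, and a timer destroys it after a few seconds.
; Overlapping an actor tagged "player" destroys the bullet and calls OnTakeAnyDamageEvent with fixed damage on player 0's BP_ThirdPersonCharacter, rather than on the overlapped actor.
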(event Custom|Destroy
  (Actor|DestroyActor))

(event EventBeginPlay
  (Utilities|Time|SetTimerbyEvent (delegate Custom|Destroy) 5.0 true))

(event EventTick
  (params (DeltaSeconds :type Float%20%28single-precision%29))
  (Transformation|SetActorLocation (+ (Transformation|GetActorLocation) (* (* DeltaSeconds (Variables|Default|GetSpeed)) (Transformation|GetActorForwardVector))) false false))

(event Collision|EventActorBeginOverlap
  (params (OtherActor :type Actor%20Object%20Reference))
  (if (Utilities|Array|ContainsItem (Variables|/Script/Engine.Actor|GetTags OtherActor) "player")
    (Actor|DestroyActor)
    (bind _asbp_third_person_character (Utilities|Casting|CastToBP_ThirdPersonCharacter (Game|GetPlayerCharacter 0)))
    (Default|OnTakeAnyDamageEvent _asbp_third_person_character 0 1e+01)))

(fn ConstructionScript)